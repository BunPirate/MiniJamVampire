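; BP_EnemyBase is the base enemy character, which shoots projectiles and takes damage until it dies.
; A timer set on BeginPlay calls SpawnProj, which launches a non-bouncing BP_EnemyProjectile, aiming its rotation at the player capsule's forward vector rather than its location.
; DoDamage spawns damage-scaled floating text, applies knockback through LaunchCharacter, reduces Health and destroys the actor through Die when Health runs out.
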(event Custom|Die
  (Actor|DestroyActor))

(event Custom|shooting
  (CallFunction|SpawnProj))

(event EventBeginPlay
  (Utilities|Time|SetTimerbyEvent (delegate Custom|shooting) 5.0))

(fn ConstructionScript)

(fn SpawnProj
  (bind _sprite (Variables|Default|GetSprite))
  (bind _returnvalue (Transformation|GetWorldLocation _sprite))
  (bind _returnvalue_2 (Game|SpawnActorfromClass "/Game/Blueprints/Projectiles/BP_EnemyProjectile.BP_EnemyProjectile_C" (Math|Transform|MakeTransform (+ _returnvalue (Math|Vector|GetForwardVector _sprite)) (Math|Rotator|FindLookatRotation _returnvalue (Math|Vector|GetForwardVector (Variables|/Script/Engine.Character|GetCapsuleComponent (Game|GetPlayerCharacter 0)))) "1.000000,1.000000,1.000000") "AdjustIfPossibleButAlwaysSpawn" 0 0))
  (Game|Components|ProjectileMovement|SetVelocityinLocalSpace (Variables|/Game/Blueprints/Projectiles/BP_EnemyProjectile.BP_EnemyProjectile_C|GetProjectileMovement _returnvalue_2) (* (Transformation|GetActorForwardVector) 1e+02))
  (Default|InitializeProjectile _returnvalue_2 0 4e+01 false)
  (return))

(fn DoDamage
  (params (Damage :type Float%20%28double-precision%29) (ImpulseVelocity :type Vector :default "0, 0, 0"))
  (bind _returnvalue (Game|SpawnActorfromClass "/Game/Blueprints/UI/BP_FloatingText.BP_FloatingText_C" (Math|Transform|MakeTransform (.location (Transformation|GetWorldTransform (Variables|Collision|GetCapsuleComponent))) "0, 0, 0" (Math|Conversions|ToVector(Float) (Math|Float|MapRangeClamped Damage 1e+01 5e+02 0.5 2.0))) "Undefined" 0 0))
  (Default|SpawnFloatingText _returnvalue "NewEnumerator1" (Utilities|Text|ToText(Float) Damage "HalfToEven"))
  (Character|LaunchCharacter ImpulseVelocity false false)
  (Variables|Default|SetHealth (- (Variables|Default|GetHealth) Damage))
  (if (> (Variables|Default|GetHealth) 0.0)
    (return self 0)
    (else
      (CallFunction|Die)
      (return self 0))))