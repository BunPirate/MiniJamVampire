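; Level generator Blueprint that builds a random 2D tile level at BeginPlay using a random-walk (drunkard's walk) algorithm.
; One walker steps from the origin in cardinal directions for a random lifespan, writing floor tiles into a coordinate-keyed map.
; SpawnWalls fills empty cells around each floor tile, diagonals included, with walls.
; All tiles then render as sprite instances on the XZ plane through FloorSprites, walls included.
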(event EventBeginPlay
  (bind _tilesize (Variables|Default|GetTileSize))
  (CallFunction|SpawnWalker (Utilities|Struct|MakeIntVector2 0 0) (Math|Random|RandomIntegerinRange 5000 10000))
  (CallFunction|SpawnWalls)
  ;[1 1 1] Render tiles
  (bind _values (Utilities|Map|Values (Variables|Default|GetTiles)))
  (for _array_element _values
    (Components|InstancedStaticMesh|AddInstance (Variables|Default|GetFloorSprites) (Math|Transform|MakeTransform (Math|Vector|MakeVector (Math|Conversions|ToFloat(Integer) (* (.Y (Utilities|Struct|BreakIntVector2 (.Coordinate (Utilities|Struct|BreakS_TileData _array_element)))) _tilesize)) 0.0 (Math|Conversions|ToFloat(Integer) (* (.X (Utilities|Struct|BreakIntVector2 (.Coordinate (Utilities|Struct|BreakS_TileData _array_element)))) _tilesize))) "0, 0, 0" "1.000000,1.000000,1.000000") (.Sprite (Utilities|Struct|BreakS_TileData _array_element)))))

(fn ConstructionScript)

(fn SpawnWalker
  (params (StartPosition :type Int%20Vector%202%20Structure) (Lifespan :type Integer))
  (bind _output_get (LocalVariables|SetWalkerCurrentPos StartPosition))
  (LocalVariables|SetLifeSpanLeft Lifespan)
  (CallFunction|SetTile "NewEnumerator0" _output_get)
  (while (> (LocalVariables|GetLifeSpanLeft) 0)
    (Math|Integer|DecrementInt (LocalVariables|GetLifeSpanLeft)
      (:%20%20
        (bind _newposition (CallFunction|RandomTileinDirection (LocalVariables|GetWalkerCurrentPos)))
        (bind _output_get_2 (LocalVariables|SetWalkerCurrentPos _newposition))
        (CallFunction|SetTile "NewEnumerator0" _output_get_2))))
  (return))

(fn RandomTileinDirection
  (params (Position :type Int%20Vector%202%20Structure))
  (bind (_x _y) (Utilities|Struct|BreakIntVector2 Position))
  (bind (_x_2 _y_2) (Utilities|Struct|BreakIntVector2 Position))
  (bind (_x_3 _y_3) (Utilities|Struct|BreakIntVector2 Position))
  (bind (_x_4 _y_4) (Utilities|Struct|BreakIntVector2 Position))
  (switch Utilities|FlowControl|Switch|SwitchonE_Direction (Utilities|Enum|ByteToEnumE_Direction (Math|Conversions|ToByte(Integer) (Math|Random|RandomIntegerinRange 0 3)))
    (:NewEnumerator0
      (return (Utilities|Struct|MakeIntVector2 _x_2 (+ _y_2 1))))
    (:NewEnumerator1
      (return (Utilities|Struct|MakeIntVector2 (+ _x 1) _y)))
    (:NewEnumerator2
      (return (Utilities|Struct|MakeIntVector2 _x_4 (+ _y_4 -1))))
    (:NewEnumerator3
      (return (Utilities|Struct|MakeIntVector2 (+ _x_3 -1) _y_3)))))

(fn SetTile
  (params (TileType :type E_TileType%20Enum :default "NewEnumerator0") (Position :type Int%20Vector%202%20Structure))
  (Utilities|Map|Add (Variables|Default|GetTiles) Position (Utilities|Struct|MakeS_TileData (Utilities|Select :Index TileType :NewEnumerator0 "/Game/Sprites/Floor.Floor" :NewEnumerator1 "/Game/Sprites/Wall.Wall") TileType Position)))

(fn SpawnWalls
  (bind _values (Utilities|Map|Values (Variables|Default|GetTiles)))
  (for _array_element _values
    (switch Utilities|FlowControl|Switch|SwitchonE_TileType (.Type (Utilities|Struct|BreakS_TileData _array_element))
      (:NewEnumerator0
        (bind _surroundingtiles (CallFunction|GetNeighboringTiles (.Coordinate (Utilities|Struct|BreakS_TileData _array_element))))
        (for _array_element_2 _surroundingtiles
          (if (not (.ReturnValue (Utilities|Map|Find (Variables|Default|GetTiles) _array_element_2)))
            (CallFunction|SetTile "NewEnumerator1" _array_element_2)))))))

(fn GetNeighboringTiles
  (params (CenterTile :type Int%20Vector%202%20Structure))
  (bind (_x _y) (Utilities|Struct|BreakIntVector2 CenterTile))
  (for _index (range -1 1)
    (for _index_2 (range -1 1)
      (Utilities|Array|AddUnique (LocalVariables|GetTiles) (Utilities|Struct|MakeIntVector2 (+ _index _x) (+ _index_2 _y)))))
  (return (LocalVariables|GetTiles)))