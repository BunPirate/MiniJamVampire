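; Health-up item that raises the interacting player's maximum health by a fixed amount.
; Interact rebuilds the player's CharacterStats struct with increased MaxHealth, copying current health and the other stats unchanged, then destroys the item.
; A debug print follows, but it re-adds the bonus to the already updated value, so it overstates the new maximum.
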(fn ConstructionScript
  (|CallParentFunction))

(fn Interact
  (params (PlayerRef :type BP%20Character%20Object%20Reference))
  (Variables|/Game/Blueprints/BP_Character.BP_Character_C|SetCharacterStats PlayerRef (Utilities|Struct|MakeS_CharacterStats (+ (.MaxHealth (Utilities|Struct|BreakS_CharacterStats (Variables|/Game/Blueprints/BP_Character.BP_Character_C|GetCharacterStats PlayerRef))) 1e+01) (.CurrentHealth (Utilities|Struct|BreakS_CharacterStats (Variables|/Game/Blueprints/BP_Character.BP_Character_C|GetCharacterStats PlayerRef))) (.Speed (Utilities|Struct|BreakS_CharacterStats (Variables|/Game/Blueprints/BP_Character.BP_Character_C|GetCharacterStats PlayerRef))) (.FireDelay (Utilities|Struct|BreakS_CharacterStats (Variables|/Game/Blueprints/BP_Character.BP_Character_C|GetCharacterStats PlayerRef))) (.Damage (Utilities|Struct|BreakS_CharacterStats (Variables|/Game/Blueprints/BP_Character.BP_Character_C|GetCharacterStats PlayerRef))) (.Knockback (Utilities|Struct|BreakS_CharacterStats (Variables|/Game/Blueprints/BP_Character.BP_Character_C|GetCharacterStats PlayerRef))) (.ProjectileSize (Utilities|Struct|BreakS_CharacterStats (Variables|/Game/Blueprints/BP_Character.BP_Character_C|GetCharacterStats PlayerRef))) (.MaxBounces (Utilities|Struct|BreakS_CharacterStats (Variables|/Game/Blueprints/BP_Character.BP_Character_C|GetCharacterStats PlayerRef))) (.ProjectileSpeed (Utilities|Struct|BreakS_CharacterStats (Variables|/Game/Blueprints/BP_Character.BP_Character_C|GetCharacterStats PlayerRef))) (.RollCooldown (Utilities|Struct|BreakS_CharacterStats (Variables|/Game/Blueprints/BP_Character.BP_Character_C|GetCharacterStats PlayerRef)))))
  (Actor|DestroyActor)
  (Development|PrintString (Utilities|String|Append "Max health is now: " (Utilities|String|ToString(Float) (+ (.MaxHealth (Utilities|Struct|BreakS_CharacterStats (Variables|/Game/Blueprints/BP_Character.BP_Character_C|GetCharacterStats PlayerRef))) 1e+01))))
  (return 0))