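; BP_ItemBase is a base item actor that a player picks up by interacting with it.
; Interact stores the player reference and destroys the item, without applying any stats itself.
; A separate AddToStats event adds a supplied stats struct field by field to the stored player's CharacterStats, covering health, movement, roll cooldown and projectile combat values.
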(event Custom|AddToStats
  (params (StatsToAdd :type S%20Character%20Stats%20Structure%20%28by%20ref%29))
  (bind (_maxhealth _currenthealth _speed _firedelay _damage _knockback _projectilesize _maxbounces _projectilespeed _rollcooldown _shots _crit) (Utilities|Struct|BreakS_CharacterStats StatsToAdd))
  (Variables|/Game/Blueprints/BP_Character.BP_Character_C|SetCharacterStats (Variables|Default|GetPlayer%20Ref) (Utilities|Struct|MakeS_CharacterStats (+ _maxhealth (.MaxHealth (Utilities|Struct|BreakS_CharacterStats (Variables|/Game/Blueprints/BP_Character.BP_Character_C|GetCharacterStats (Variables|Default|GetPlayer%20Ref))))) (+ _currenthealth (.CurrentHealth (Utilities|Struct|BreakS_CharacterStats (Variables|/Game/Blueprints/BP_Character.BP_Character_C|GetCharacterStats (Variables|Default|GetPlayer%20Ref))))) (+ _speed (.Speed (Utilities|Struct|BreakS_CharacterStats (Variables|/Game/Blueprints/BP_Character.BP_Character_C|GetCharacterStats (Variables|Default|GetPlayer%20Ref))))) (+ _firedelay (.FireDelay (Utilities|Struct|BreakS_CharacterStats (Variables|/Game/Blueprints/BP_Character.BP_Character_C|GetCharacterStats (Variables|Default|GetPlayer%20Ref))))) (+ _damage (.Damage (Utilities|Struct|BreakS_CharacterStats (Variables|/Game/Blueprints/BP_Character.BP_Character_C|GetCharacterStats (Variables|Default|GetPlayer%20Ref))))) (+ _knockback (.Knockback (Utilities|Struct|BreakS_CharacterStats (Variables|/Game/Blueprints/BP_Character.BP_Character_C|GetCharacterStats (Variables|Default|GetPlayer%20Ref))))) (+ _projectilesize (.ProjectileSize (Utilities|Struct|BreakS_CharacterStats (Variables|/Game/Blueprints/BP_Character.BP_Character_C|GetCharacterStats (Variables|Default|GetPlayer%20Ref))))) (+ _maxbounces (.MaxBounces (Utilities|Struct|BreakS_CharacterStats (Variables|/Game/Blueprints/BP_Character.BP_Character_C|GetCharacterStats (Variables|Default|GetPlayer%20Ref))))) (+ _projectilespeed (.ProjectileSpeed (Utilities|Struct|BreakS_CharacterStats (Variables|/Game/Blueprints/BP_Character.BP_Character_C|GetCharacterStats (Variables|Default|GetPlayer%20Ref))))) (+ _rollcooldown (.RollCooldown (Utilities|Struct|BreakS_CharacterStats (Variables|/Game/Blueprints/BP_Character.BP_Character_C|GetCharacterStats (Variables|Default|GetPlayer%20Ref))))) (+ _shots (.Shots (Utilities|Struct|BreakS_CharacterStats (Variables|/Game/Blueprints/BP_Character.BP_Character_C|GetCharacterStats (Variables|Default|GetPlayer%20Ref))))) (+ _crit (.Crit (Utilities|Struct|BreakS_CharacterStats (Variables|/Game/Blueprints/BP_Character.BP_Character_C|GetCharacterStats (Variables|Default|GetPlayer%20Ref))))))))

(fn ConstructionScript)

(fn Interact
  (params (PlayerRef :type BP%20Character%20Object%20Reference))
  (Variables|Default|SetPlayer%20Ref PlayerRef)
  (Actor|DestroyActor)
  (return 0))