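; Enemy projectile that sends a damage message with velocity-scaled knockback to whatever it hits, then destroys itself.
; InitializeProjectile stores damage and a bounce count, recolors the light cyan on crits, and starts the lifetime timer.
; A timeline animates the light's intensity, then hides it.
; When the timer expires, Kill shrinks the sphere to zero through a second timeline before destroying the actor.
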(event Custom|Kill
  (Utilities|Time|ClearandInvalidateTimerbyHandle (Variables|Default|GetTimer))
  (bind _yeet (Timeline|DieTimer Play)
    (:Update
      (Transformation|SetRelativeScale3D (Variables|Default|GetSphere) (Math|Vector|Lerp(Vector) "1.000000,1.000000,1.000000" "0, 0, 0" _yeet)))
    (:Finished
      (Actor|DestroyActor))))

(event Custom|InitializeProjectile
  (params (MaxBounces :type Integer) (Damage :type Float%20%28double-precision%29) (IsCrit :type Boolean))
  (bind _pointlight (Variables|Default|GetPointLight))
  (if IsCrit
    (Rendering|Components|Light|SetIntensity _pointlight 1e+03)
    (Rendering|Components|Light|SetLightColor _pointlight "(R=0.059669,G=0.930299,B=1.000000,A=1.000000)" true))
  (Variables|Default|SetDamage Damage)
  (Variables|Default|SetBounces MaxBounces)
  (bind _returnvalue (Utilities|Time|SetTimerbyEvent (delegate Custom|Kill) 25.0))
  (Variables|Default|SetTimer _returnvalue)
  (bind _yeet (Timeline|LightTimer Play)
    (:Update
      (Rendering|Components|Light|SetIntensity (Variables|Default|GetPointLight) (Math|Float|Lerp 0.0 1e+03 _yeet)))
    (:Finished
      (Rendering|SetVisibility (Variables|Default|GetPointLight) false false))))

(event Collision|EventHit
  (params (MyComp :type Primitive%20Component%20Object%20Reference) (Other :type Actor%20Object%20Reference) (OtherComp :type Primitive%20Component%20Object%20Reference) (bSelfMoved :type Boolean) (HitLocation :type Vector :default "0, 0, 0") (HitNormal :type Vector :default "0, 0, 0") (NormalImpulse :type Vector :default "0, 0, 0") (Hit :type Hit%20Result%20Structure%20%28by%20ref%29))
  (Class|BPIDamage|DoDamage(Message) Other (Variables|Default|GetDamage) (* (Transformation|GetVelocity) (Variables|Default|GetKnockbackForce)))
  (Actor|DestroyActor))

(fn ConstructionScript)