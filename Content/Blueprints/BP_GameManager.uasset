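; BP_GameManager tracks the current game stage and handles advancing to the next one.
; On BeginPlay it caches BP_GameInstance and copies its GameStage, so the count survives level loads.
; NextLevel increments the stage, writes it back to the game instance and opens L_Test, the same map for every stage.
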(event Custom|NextLevel
  (bind _result (Math|Integer|IncrementInt (Variables|Default|GetGame%20Stage))
    (:%20%20
      (Variables|/Game/Blueprints/GamemodeStuff/BP_GameInstance.BP_GameInstance_C|SetGameStage (Variables|Default|GetAs%20BP%20Game%20Instance) _result)
      (Game|OpenLevel(byObjectReference) "/Game/Levels/L_Test.L_Test"))))

(event EventBeginPlay
  (bind _asbp_game_instance (Utilities|Casting|CastToBP_GameInstance (Game|GetGameInstance)))
  (bind _output_get (Variables|Default|SetAs%20BP%20Game%20Instance _asbp_game_instance))
  (Variables|Default|SetGame%20Stage (Variables|/Game/Blueprints/GamemodeStuff/BP_GameInstance.BP_GameInstance_C|GetGameStage _output_get)))

(fn ConstructionScript)