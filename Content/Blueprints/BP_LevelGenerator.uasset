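; Procedural level generator that builds a random tile map on BeginPlay, scaled and themed by the game instance's GameStage.
; A random walker carves floor tiles into a map, with lifespan growing per stage, then leaves a goal at its endpoint, or a boss on stage 5.
; Walls ring the floor, tiles render as instanced area sprites (random area past stage 5) plus wall meshes, and enemies spawn by per-tile chance.
; Item spawning exists but is unwired.
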(event EventBeginPlay
  (bind _tilesize (Variables|Default|GetTileSize))
  (bind _asbp_game_instance (Utilities|Casting|CastToBP_GameInstance (Game|GetGameInstance)))
  (Variables|Default|SetAs%20BP%20Game%20Instance _asbp_game_instance)
  (CallFunction|SpawnWalker (Utilities|Struct|MakeIntVector2 0 0) (+ (Variables|Default|GetMaxSteps) (* (+ (Variables|/Game/Blueprints/GamemodeStuff/BP_GameInstance.BP_GameInstance_C|GetGameStage (Variables|Default|GetAs%20BP%20Game%20Instance)) 1) 100)))
  (CallFunction|SpawnWalls)
  (Variables|Default|SetRandomStage (Math|Random|RandomIntegerinRange 0 (Variables|Default|GetMaxStages)))
  ;[1 1 1] Render tiles
  (bind _values (Utilities|Map|Values (Variables|Default|GetTiles)))
  (for _array_element _values
    (Components|InstancedStaticMesh|AddInstance (Variables|Default|GetWallSprites) (Math|Transform|MakeTransform (Math|Vector|MakeVector (Math|Conversions|ToFloat(Integer) (* (.Y (Utilities|Struct|BreakIntVector2 (.Coordinate (Utilities|Struct|BreakS_TileData _array_element)))) _tilesize)) (Utilities|Select :Index (.Type (Utilities|Struct|BreakS_TileData _array_element)) :NewEnumerator0 0.0 :NewEnumerator1 5e+01) (Math|Conversions|ToFloat(Integer) (* (.X (Utilities|Struct|BreakIntVector2 (.Coordinate (Utilities|Struct|BreakS_TileData _array_element)))) _tilesize))) "0, 0, 0" "1.000000,1.000000,1.000000") (.OutItem (Utilities|Array|Random (Utilities|Select :Index (.Type (Utilities|Struct|BreakS_TileData _array_element)) :NewEnumerator0 (Utilities|Select :Index (Math|Integer|SelectInt (Variables|Default|GetRandomStage) (Variables|/Game/Blueprints/GamemodeStuff/BP_GameInstance.BP_GameInstance_C|GetGameStage (Variables|Default|GetAs%20BP%20Game%20Instance)) (> (Variables|/Game/Blueprints/GamemodeStuff/BP_GameInstance.BP_GameInstance_C|GetGameStage (Variables|Default|GetAs%20BP%20Game%20Instance)) 5)) :Option%200 (Variables|Default|GetArea0Floor) :Option%201 (Variables|Default|GetArea1Floor) :Option%202 (Variables|Default|GetArea2Floor) :Option%203 (Variables|Default|GetArea3Floor) :Option%204 (Variables|Default|GetArea4Floor) :Option%205 (Variables|Default|GetArea5Floor)) :NewEnumerator1 (Utilities|Select :Index (Math|Integer|SelectInt (Variables|Default|GetRandomStage) (Variables|/Game/Blueprints/GamemodeStuff/BP_GameInstance.BP_GameInstance_C|GetGameStage (Variables|Default|GetAs%20BP%20Game%20Instance)) (> (Variables|/Game/Blueprints/GamemodeStuff/BP_GameInstance.BP_GameInstance_C|GetGameStage (Variables|Default|GetAs%20BP%20Game%20Instance)) 5)) :Option%200 (Variables|Default|GetArea0Wall) :Option%201 (Variables|Default|GetArea1Wall) :Option%202 (Variables|Default|GetArea2Wall) :Option%203 (Variables|Default|GetArea3Wall) :Option%204 (Variables|Default|GetArea4Wall) :Option%205 (Variables|Default|GetArea5Wall))))))
    (switch Utilities|FlowControl|Switch|SwitchonE_TileType (.Type (Utilities|Struct|BreakS_TileData _array_element))
      (:NewEnumerator1
        (Components|InstancedStaticMesh|AddInstance (Variables|Default|GetInstancedStaticMesh) (Math|Transform|MakeTransform (Math|Vector|MakeVector (Math|Conversions|ToFloat(Integer) (* (.X (Utilities|Struct|BreakIntVector2 (.Coordinate (Utilities|Struct|BreakS_TileData _array_element)))) _tilesize)) (Math|Conversions|ToFloat(Integer) (* (.Y (Utilities|Struct|BreakIntVector2 (.Coordinate (Utilities|Struct|BreakS_TileData _array_element)))) _tilesize)) -1.5) "0, 0, 0" "0.400000,0.400000,0.400000") true))))
  (CallFunction|EnemySpawn))

(fn ConstructionScript)

(fn SpawnWalker
  (params (StartPosition :type Int%20Vector%202%20Structure) (Lifespan :type Integer))
  (bind _output_get (LocalVariables|SetWalkerCurrentPos StartPosition))
  (LocalVariables|SetLifeSpanLeft Lifespan)
  (CallFunction|SetTile "NewEnumerator0" _output_get)
  (while (> (LocalVariables|GetLifeSpanLeft) 0)
    (Math|Integer|DecrementInt (LocalVariables|GetLifeSpanLeft)
      (:%20%20
        (bind _newposition (CallFunction|RandomTileinDirection (LocalVariables|GetWalkerCurrentPos)))
        (bind _output_get_2 (LocalVariables|SetWalkerCurrentPos _newposition))
        (CallFunction|SetTile "NewEnumerator0" _output_get_2))))
  (if (== (Variables|/Game/Blueprints/GamemodeStuff/BP_GameInstance.BP_GameInstance_C|GetGameStage (Variables|Default|GetAs%20BP%20Game%20Instance)) 5)
    (Game|SpawnActorfromClass "/Game/Enemies/EnemyBoss.EnemyBoss_C" (Math|Transform|MakeTransform (Math|Vector|MakeVector (* (Math|Conversions|ToFloat(Integer) (.x (LocalVariables|GetWalkerCurrentPos))) 1e+02) (* (Math|Conversions|ToFloat(Integer) (.y (LocalVariables|GetWalkerCurrentPos))) 1e+02) 5e+01) "0, 0, 0" "1.000000,1.000000,1.000000") "AdjustIfPossibleButAlwaysSpawn" 0 0)
    (return)
    (else
      (Game|SpawnActorfromClass "/Game/Blueprints/BP_Goal.BP_Goal_C" (Math|Transform|MakeTransform (Math|Vector|MakeVector (* (Math|Conversions|ToFloat(Integer) (.x (LocalVariables|GetWalkerCurrentPos))) 1e+02) (* (Math|Conversions|ToFloat(Integer) (.y (LocalVariables|GetWalkerCurrentPos))) 1e+02) 0.0) "0, 0, 0" "1.000000,1.000000,1.000000") "Undefined" 0 0))))

(fn RandomTileinDirection
  (params (Position :type Int%20Vector%202%20Structure))
  (bind (_x _y) (Utilities|Struct|BreakIntVector2 Position))
  (bind (_x_2 _y_2) (Utilities|Struct|BreakIntVector2 Position))
  (bind (_x_3 _y_3) (Utilities|Struct|BreakIntVector2 Position))
  (bind (_x_4 _y_4) (Utilities|Struct|BreakIntVector2 Position))
  (switch Utilities|FlowControl|Switch|SwitchonE_Direction (Utilities|Enum|ByteToEnumE_Direction (Math|Conversions|ToByte(Integer) (Math|Random|RandomIntegerinRange 0 3)))
    (:NewEnumerator0
      (return (Utilities|Struct|MakeIntVector2 _x_2 (+ _y_2 1))))
    (:NewEnumerator1
      (return (Utilities|Struct|MakeIntVector2 (+ _x 1) _y)))
    (:NewEnumerator2
      (return (Utilities|Struct|MakeIntVector2 _x_4 (+ _y_4 -1))))
    (:NewEnumerator3
      (return (Utilities|Struct|MakeIntVector2 (+ _x_3 -1) _y_3)))))

(fn SetTile
  (params (TileType :type E_TileType%20Enum :default "NewEnumerator0") (Position :type Int%20Vector%202%20Structure))
  (Utilities|Map|Add (Variables|Default|GetTiles) Position (Utilities|Struct|MakeS_TileData (Utilities|Select :Index TileType :NewEnumerator0 "/Game/Sprites/Tiles/Floor.Floor" :NewEnumerator1 "/Game/Sprites/Tiles/Wall.Wall") TileType Position)))

(fn SpawnWalls
  (bind _values (Utilities|Map|Values (Variables|Default|GetTiles)))
  (for _array_element _values
    (switch Utilities|FlowControl|Switch|SwitchonE_TileType (.Type (Utilities|Struct|BreakS_TileData _array_element))
      (:NewEnumerator0
        (bind _surroundingtiles (CallFunction|GetNeighboringTiles (.Coordinate (Utilities|Struct|BreakS_TileData _array_element))))
        (for _array_element_2 _surroundingtiles
          (if (not (.ReturnValue (Utilities|Map|Find (Variables|Default|GetTiles) _array_element_2)))
            (CallFunction|SetTile "NewEnumerator1" _array_element_2)))))))

(fn GetNeighboringTiles
  (params (CenterTile :type Int%20Vector%202%20Structure))
  (bind (_x _y) (Utilities|Struct|BreakIntVector2 CenterTile))
  (for _index (range -1 1)
    (for _index_2 (range -1 1)
      (Utilities|Array|AddUnique (LocalVariables|GetTiles) (Utilities|Struct|MakeIntVector2 (+ _index _x) (+ _index_2 _y)))))
  (return (LocalVariables|GetTiles)))

(fn EnemySpawn
  (bind _values (Utilities|Map|Values (Variables|Default|GetTiles)))
  (for _array_element _values
    (switch Utilities|FlowControl|Switch|SwitchonE_TileType (.Type (Utilities|Struct|BreakS_TileData _array_element))
      (:NewEnumerator0
        (if (Math|Random|RandomBoolwithWeight (Variables|Default|GetEnemy%20Spawn%20chance))
          (Game|SpawnActorfromClass "/Game/Enemies/BP_EnemyBase.BP_EnemyBase_C" (Math|Transform|MakeTransform (Math|Vector|MakeVector (* (Math|Conversions|ToFloat(Integer) (.X (Utilities|Struct|BreakIntVector2 (.Coordinate (Utilities|Struct|BreakS_TileData _array_element))))) 1e+02) (* (Math|Conversions|ToFloat(Integer) (.Y (Utilities|Struct|BreakIntVector2 (.Coordinate (Utilities|Struct|BreakS_TileData _array_element))))) 1e+02) 1e+02) "0, 0, 0" "1.000000,1.000000,1.000000") "Undefined" 0 0))))))

(fn SpawnItems
  (bind _values (Utilities|Map|Values (Variables|Default|GetTiles)))
  (for _array_element _values
    (switch Utilities|FlowControl|Switch|SwitchonE_TileType (.Type (Utilities|Struct|BreakS_TileData _array_element))
      (:NewEnumerator0
        (if (Math|Random|RandomBoolwithWeight (Variables|Default|GetItemSpawnChance))
          (Game|SpawnActorfromClass (.OutItem (Utilities|Array|Random (Variables|Default|GetPotentialItems))) (Math|Transform|MakeTransform (Math|Vector|MakeVector (* (Math|Conversions|ToFloat(Integer) (.X (Utilities|Struct|BreakIntVector2 (.Coordinate (Utilities|Struct|BreakS_TileData _array_element))))) 1e+02) (* (Math|Conversions|ToFloat(Integer) (.Y (Utilities|Struct|BreakIntVector2 (.Coordinate (Utilities|Struct|BreakS_TileData _array_element))))) 1e+02) 0.0) "0, 0, 0" "1.000000,1.000000,1.000000") "Undefined" 0 0))))))