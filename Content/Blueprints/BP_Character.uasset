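; Player character with a sprite that moves on the world XY plane and uses a crosshair as the mouse cursor.
; On BeginPlay it shows the mouse cursor and replaces the default one with a W_Crosshair widget.
; Horizontal and Vertical axis inputs add movement along world X and negative Y.
; Tick mirrors the sprite through its X scale according to horizontal velocity, keeping the last facing when nearly still.
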(event EventTick
  (params (DeltaSeconds :type Float%20%28single-precision%29))
  (bind _returnvalue (Transformation|GetVelocity))
  (bind _sprite (Variables|Default|GetSprite))
  (if (> (.x _returnvalue) 0.1)
    (Transformation|SetRelativeScale3D _sprite "1.000000,1.000000,1.000000")
    (elif (< (.x _returnvalue) -0.1)
      (Transformation|SetRelativeScale3D _sprite "-1.000000,1.000000,1.000000"))))

(event EventBeginPlay
  (bind _returnvalue (Game|GetPlayerController 0))
  (Variables|/Script/Engine.PlayerController|SetbShowMouseCursor _returnvalue true)
  (bind _returnvalue_2 (UserInterface|CreateWidget "/Game/Sprites/Textures/W_Crosshair.W_Crosshair_C"))
  (Class|PlayerController|SetMouseCursorWidget _returnvalue "Default" _returnvalue_2))

(event Input|AxisEvents|InputAxisHorizontal
  (params (AxisValue :type Float%20%28single-precision%29))
  (Pawn|Input|AddMovementInput "1.000000, 0, 0" AxisValue false)
  (if (> AxisValue 0.1)
    _))

(event Input|AxisEvents|InputAxisVertical
  (params (AxisValue :type Float%20%28single-precision%29))
  (Pawn|Input|AddMovementInput "0.000000,-1.000000, 0" AxisValue false))

(fn ConstructionScript)